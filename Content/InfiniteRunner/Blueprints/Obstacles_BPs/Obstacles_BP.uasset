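; Obstacle actor for the infinite runner that either kills the player or consumes their shield on contact.
; Its box collision overlap with the player character checks the shield flag on the ThirdPersonGameMode.
; An active shield is switched off, a break sound plays and the obstacle destroys itself; otherwise it calls Death on the player character.
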(event OnComponentBeginOverlap(BoxCollision)
  (params (OverlappedComponent :type Primitive%20Component%20Object%20Reference) (OtherActor :type Actor%20Object%20Reference) (OtherComp :type Primitive%20Component%20Object%20Reference) (OtherBodyIndex :type Integer) (bFromSweep :type Boolean) (SweepResult :type Hit%20Result%20Structure%20%28by%20ref%29))
  (if (== OtherActor (Game|GetPlayerCharacter 0))
    (CallFunction|KillPlayerorShield)))

(fn ConstructionScript)

(fn KillPlayerorShield
  (bind _asthird_person_game_mode (Utilities|Casting|CastToThirdPersonGameMode (Game|GetGameMode)))
  (if (Variables|/Game/InfiniteRunner/ThirdPersonBP/Blueprints/ThirdPersonGameMode.ThirdPersonGameMode_C|GetIsShieldOn _asthird_person_game_mode)
    (Variables|/Game/InfiniteRunner/ThirdPersonBP/Blueprints/ThirdPersonGameMode.ThirdPersonGameMode_C|SetIsShieldOn _asthird_person_game_mode false)
    (Audio|PlaySound2D "/Game/InfiniteRunner/Sounds/break06-36414.break06-36414" 1.0 1.0 0.0 0 0)
    (Actor|DestroyActor)
    (else
      (bind _asthird_person_character (Utilities|Casting|CastToThirdPersonCharacter (Game|GetPlayerCharacter 0)))
      (Default|Death _asthird_person_character))))