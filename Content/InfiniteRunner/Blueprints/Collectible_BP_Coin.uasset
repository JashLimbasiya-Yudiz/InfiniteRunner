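; Coin pickup for an infinite runner that adds to the game mode's coin count and destroys itself when the player overlaps it.
; Pickup loads the SaveGame slot to check the Sound setting before playing a coin sound.
; While the player is inside the magnet sphere with the game mode's magnet on, Tick restarts a timeline that interpolates the coin toward the player, adding a Transition offset.
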(event OnComponentBeginOverlap(SphereCollision)
  (params (OverlappedComponent :type Primitive%20Component%20Object%20Reference) (OtherActor :type Actor%20Object%20Reference) (OtherComp :type Primitive%20Component%20Object%20Reference) (OtherBodyIndex :type Integer) (bFromSweep :type Boolean) (SweepResult :type Hit%20Result%20Structure%20%28by%20ref%29))
  (if (== OtherActor (Game|GetPlayerCharacter 0))
    (bind _asthird_person_game_mode (Utilities|Casting|CastToThirdPersonGameMode (Game|GetGameMode)))
    (Variables|/Game/InfiniteRunner/ThirdPersonBP/Blueprints/ThirdPersonGameMode.ThirdPersonGameMode_C|SetCoins _asthird_person_game_mode (+ (Variables|/Game/InfiniteRunner/ThirdPersonBP/Blueprints/ThirdPersonGameMode.ThirdPersonGameMode_C|GetCoins _asthird_person_game_mode) 1))
    (Actor|DestroyActor)
    (bind _returnvalue (SaveGame|LoadGamefromSlot "SaveGame"))
    (bind _asinfinite_runner_save_game (Utilities|Casting|CastToInfiniteRunnerSaveGame _returnvalue))
    (if (Variables|/Game/InfiniteRunner/Blueprints/InfiniteRunnerSaveGame.InfiniteRunnerSaveGame_C|GetSound _asinfinite_runner_save_game)
      (Audio|PlaySound2D "/Game/InfiniteRunner/Sounds/350874__cabled_mess__coin_c_08.350874__cabled_mess__coin_c_08" 1.0 1.0 0.0 0 0))))

(event EventTick
  (params (DeltaSeconds :type Float%20%28single-precision%29))
  (if (Collision|IsOverlappingActor (Variables|Default|GetSphereForMagnet) (Game|GetPlayerCharacter 0) :!class /Script/Engine.PrimitiveComponent)
    (bind _asthird_person_game_mode (Utilities|Casting|CastToThirdPersonGameMode (Game|GetGameMode)))
    (if (Variables|/Game/InfiniteRunner/ThirdPersonBP/Blueprints/ThirdPersonGameMode.ThirdPersonGameMode_C|GetIsMegnateOn _asthird_person_game_mode)
      (bind _transition (Timeline|Timeline PlayFromStart)
        (:Update
          (Transformation|SetActorLocation (+ _transition (Math|Interpolation|VInterpTo (.location (Transformation|GetActorTransform)) (Transformation|GetActorLocation (Game|GetPlayerCharacter 0)) (Utilities|Time|GetWorldDeltaSeconds) 2e+01)) false true))))))

(fn ConstructionScript
  (|CallParentFunction))