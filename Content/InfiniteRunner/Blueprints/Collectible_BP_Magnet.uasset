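; Magnet power-up collectible for the infinite runner, picked up when the player character overlaps its sphere collision.
; On pickup it calls ActivateMagnet on the ThirdPersonGameMode, which owns the magnet effect, and destroys itself.
; It then loads the InfiniteRunnerSaveGame slot to check the Sound setting and plays a 2D bonus sound if enabled.
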(event OnComponentBeginOverlap(SphereCollision)
  (params (OverlappedComponent :type Primitive%20Component%20Object%20Reference) (OtherActor :type Actor%20Object%20Reference) (OtherComp :type Primitive%20Component%20Object%20Reference) (OtherBodyIndex :type Integer) (bFromSweep :type Boolean) (SweepResult :type Hit%20Result%20Structure%20%28by%20ref%29))
  (if (== OtherActor (Game|GetPlayerCharacter 0))
    (bind _asthird_person_game_mode (Utilities|Casting|CastToThirdPersonGameMode (Game|GetGameMode)))
    (Default|ActivateMagnet _asthird_person_game_mode)
    (Actor|DestroyActor)
    (bind _returnvalue (SaveGame|LoadGamefromSlot "SaveGame"))
    (bind _asinfinite_runner_save_game (Utilities|Casting|CastToInfiniteRunnerSaveGame _returnvalue))
    (if (Variables|/Game/InfiniteRunner/Blueprints/InfiniteRunnerSaveGame.InfiniteRunnerSaveGame_C|GetSound _asinfinite_runner_save_game)
      (Audio|PlaySound2D "/Game/InfiniteRunner/Sounds/game-bonus-144751.game-bonus-144751" 1.0 1.0 0.0 0 0))))

(fn ConstructionScript
  (|CallParentFunction))