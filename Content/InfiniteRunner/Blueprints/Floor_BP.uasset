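; Floor tile for an infinite runner that recycles the track and randomly places obstacles across three lanes.
; When the player overlaps its Box, it removes the oldest tile from ThirdPersonGameMode's Floors array and appends a new one at the last tile's NextFloor.
; The construction script records obstacle and coin points per lane, then randomly adds obstacle child actors, capping the blocking type at two.
; Coin points are not used here, and the Lose call is unreachable.
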(event OnComponentBeginOverlap(Box)
  (params (OverlappedComponent :type Primitive%20Component%20Object%20Reference) (OtherActor :type Actor%20Object%20Reference) (OtherComp :type Primitive%20Component%20Object%20Reference) (OtherBodyIndex :type Integer) (bFromSweep :type Boolean) (SweepResult :type Hit%20Result%20Structure%20%28by%20ref%29))
  (if (== OtherActor (Game|GetPlayerCharacter 0))
    (bind _asthird_person_game_mode (Utilities|Casting|CastToThirdPersonGameMode (Game|GetGameMode)))
    (Actor|DestroyActor (Utilities|Array|Get(acopy) (Variables|/Game/InfiniteRunner/ThirdPersonBP/Blueprints/ThirdPersonGameMode.ThirdPersonGameMode_C|GetFloors _asthird_person_game_mode)))
    (Utilities|Array|RemoveIndex (Variables|/Game/InfiniteRunner/ThirdPersonBP/Blueprints/ThirdPersonGameMode.ThirdPersonGameMode_C|GetFloors _asthird_person_game_mode))
    (bind _returnvalue (Game|SpawnActorfromClass "Floor_BP_C" (Math|Transform|MakeTransform (Transformation|GetWorldLocation (Variables|Floor_BP_C|GetNextFloor (Utilities|Array|Get(acopy) (Variables|/Game/InfiniteRunner/ThirdPersonBP/Blueprints/ThirdPersonGameMode.ThirdPersonGameMode_C|GetFloors _asthird_person_game_mode) (- (Utilities|Array|Length (Variables|/Game/InfiniteRunner/ThirdPersonBP/Blueprints/ThirdPersonGameMode.ThirdPersonGameMode_C|GetFloors _asthird_person_game_mode)) 1)))) "0, 0, 0" "1,1,1") "Undefined" 0 0))
    (Utilities|Array|Insert (Variables|/Game/InfiniteRunner/ThirdPersonBP/Blueprints/ThirdPersonGameMode.ThirdPersonGameMode_C|GetFloors _asthird_person_game_mode) _returnvalue (Utilities|Array|Length (Variables|/Game/InfiniteRunner/ThirdPersonBP/Blueprints/ThirdPersonGameMode.ThirdPersonGameMode_C|GetFloors _asthird_person_game_mode)))))

(fn ConstructionScript
  (for _index (range 0 2)
    (bind _returnvalue (AddComponent|AddArrowComponent false (Math|Transform|MakeTransform (Math|Vector|MakeVector 1.8e+03 (Utilities|Array|Get(acopy) (Variables|Default|GetLanePosition) _index) 0.0) "0, 0, 0" "1,1,1")))
    (Utilities|Array|Add (Variables|Default|GetObstacleSpawnPoints) (Transformation|GetWorldTransform _returnvalue))
    (bind _returnvalue_2 (AddComponent|AddArrowComponent false (Math|Transform|MakeTransform (Math|Vector|MakeVector 8e+02 (Utilities|Array|Get(acopy) (Variables|Default|GetLanePosition) _index) 0.0) "0, 0, 0" "1,1,1")))
    (Utilities|Array|Add (Variables|Default|GetCoinsSpawnPoints) (Transformation|GetWorldTransform _returnvalue_2)))
  (CallFunction|SpawnObstacles))

(fn SpawnObstacles
  (Variables|Default|SetBlockedObstacleCount 0)
  (for _array_element (Variables|Default|GetObstacleSpawnPoints)
    (if (Math|Random|RandomBool)
      (switch int (Math|Random|RandomIntegerinRange 0 3)
        (:0
          (AddComponent|AddChildActorComponent false (Math|Transform|MakeRelativeTransform _array_element (Transformation|GetActorTransform))))
        (:1
          (AddComponent|AddChildActorComponent false (Math|Transform|MakeRelativeTransform _array_element (Transformation|GetActorTransform))))
        (:2
          (AddComponent|AddChildActorComponent false (Math|Transform|MakeRelativeTransform _array_element (Transformation|GetActorTransform))))
        (:3
          (if (< (Variables|Default|GetBlockedObstacleCount) 2)
            (AddComponent|AddChildActorComponent false (Math|Transform|MakeRelativeTransform _array_element (Transformation|GetActorTransform)))
            (Math|Integer|IncrementInt (Variables|Default|GetBlockedObstacleCount))))))))